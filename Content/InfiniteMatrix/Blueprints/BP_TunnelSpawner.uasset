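; Spawner that builds a chain of tunnel segments, each with a randomized wall and chance-based health packs, slow-down pickups and Penguin enemies.
; On BeginPlay it destroys existing tunnels, bullets, enemies and pickups, then spawns the starting segments.
; Each segment attaches at the newest one's SpawnPoint and receives references to the spawner and its spawned contents.
; Contents are scattered at random X offsets and radial Y/Z positions.
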(event `self.ReceiveBeginPlay`
  (`self.SpawnInitialTunnels`))

(fn `ModifySpawnPoint`
  (params (SpawnPoint :type "Vector Structure") (MinX :type "Float (double-precision)" :default 600.0) (MaxX :type "Float (double-precision)" :default 1400.0))
  (returns (NewSpawnPoint :type "Vector Structure"))
  (bind _returnvalue (`KismetMathLibrary.MultiplyByPi` (* (`KismetMathLibrary.RandomFloat`) 2.0)))
  (bind _returnvalue_2 (* (`KismetMathLibrary.RandomFloatInRange` 0.0 300.0) (`KismetMathLibrary.Sqrt` (`KismetMathLibrary.RandomFloat`))))
  (return (`KismetMathLibrary.MakeVector` (- SpawnPoint_X (`KismetMathLibrary.RandomFloatInRange` MinX MaxX)) (* _returnvalue_2 (`KismetMathLibrary.Cos` _returnvalue)) (* _returnvalue_2 (`KismetMathLibrary.Sin` _returnvalue)))))

(fn `RandomSpawnEnemies`
  (params (SpawnPoint :type "Vector Structure"))
  (returns (ReturnEnemies :type "Array of /Game/InfiniteMatrix/Blueprints/Penguin Object Reference"))
  (locals (Enemies :type "Array of /Game/InfiniteMatrix/Blueprints/Penguin Object Reference"))
  (if (== (`KismetMathLibrary.RandomInteger` 3) 0)
    (for _ (range (+ (`KismetMathLibrary.RandomInteger` 2) 1))
      (bind _newspawnpoint (`self.ModifySpawnPoint` SpawnPoint 200.0 1000.0))
      (bind _returnvalue (`|SpawnActorFromClass` "/Game/InfiniteMatrix/Blueprints/Penguin.Penguin_C" (`KismetMathLibrary.MakeTransform` _newspawnpoint) "Undefined" "MultiplyWithRoot" null null))
      (`KismetArrayLibrary.Array_Add` (`local.Enemies`) _returnvalue))
    (return (`local.Enemies`))))

(fn `RandomSpawnHealthPack`
  (params (SpawnPoint :type "Vector Structure"))
  (returns (HealthPack :type "/Game/InfiniteMatrix/Blueprints/HealthPack Object Reference"))
  (if (== (`KismetMathLibrary.RandomInteger` 4) 0)
    (bind _newspawnpoint (`self.ModifySpawnPoint` SpawnPoint))
    (bind _returnvalue (`|SpawnActorFromClass` "/Game/InfiniteMatrix/Blueprints/HealthPack.HealthPack_C" (`KismetMathLibrary.MakeTransform` _newspawnpoint) "Undefined" "MultiplyWithRoot" null null))
    (return _returnvalue)))

(fn `RandomSpawnSlowDown`
  (params (SpawnPoint :type "Vector Structure"))
  (returns (SlowDown :type "/Game/InfiniteMatrix/Blueprints/FbxScene_Arrow Object Reference"))
  (if (== (`KismetMathLibrary.RandomInteger` 15) 0)
    (bind _newspawnpoint (`self.ModifySpawnPoint` SpawnPoint))
    (bind _returnvalue (`|SpawnActorFromClass` "/Game/InfiniteMatrix/Blueprints/FbxScene_Arrow.FbxScene_Arrow_C" (`KismetMathLibrary.MakeTransform` _newspawnpoint) "Undefined" "MultiplyWithRoot" null null))
    (return _returnvalue)))

(fn `SpawnInitialTunnels`
  (`|ExecutionSequence`
    (:`then_0`
      (bind _outactors (`GameplayStatics.GetAllActorsOfClass` "/Game/InfiniteMatrix/Blueprints/BP_Tunnel.BP_Tunnel_C"))
      (for _array_element _outactors
        (`self.K2_DestroyActor` _array_element)))
    (:`then_1`
      (bind _outactors_2 (`GameplayStatics.GetAllActorsOfClass` "/Game/InfiniteMatrix/Blueprints/BulletProjectile.BulletProjectile_C"))
      (for _array_element_2 _outactors_2
        (`self.K2_DestroyActor` _array_element_2)))
    (:`then_2`
      (bind _outactors_3 (`GameplayStatics.GetAllActorsOfClass` "/Game/InfiniteMatrix/Blueprints/Penguin.Penguin_C"))
      (for _array_element_3 _outactors_3
        (`self.K2_DestroyActor` _array_element_3)))
    (:`then_3`
      (bind _outactors_4 (`GameplayStatics.GetAllActorsOfClass` "/Game/InfiniteMatrix/Blueprints/FbxScene_Arrow.FbxScene_Arrow_C"))
      (for _array_element_4 _outactors_4
        (`self.K2_DestroyActor` _array_element_4)))
    (:`then_4`
      (bind _outactors_5 (`GameplayStatics.GetAllActorsOfClass` "/Game/InfiniteMatrix/Blueprints/HealthPack.HealthPack_C"))
      (for _array_element_5 _outactors_5
        (`self.K2_DestroyActor` _array_element_5)))
    (:`then_5`
      (for _ (range 3)
        (`/Engine/EditorBlueprintResources/StandardMacros.IsValid` (`self.NewestTunnel`)
          (:`Is Valid`
            (`self.SpawnTunnelAtSpawnPoint`))
          (:`Is Not Valid`
            (`self.SpawnTunnel` (`self.K2_GetActorLocation` (`GameplayStatics.GetPlayerPawn` 0)))))))))

(fn `SpawnTunnel`
  (params (SpawnLocation :type "Vector Structure"))
  (`|ExecutionSequence`
    (:`then_0`
      (bind _healthpack (`self.RandomSpawnHealthPack` SpawnLocation)))
    (:`then_1`
      (bind _slowdown (`self.RandomSpawnSlowDown` SpawnLocation)))
    (:`then_2`
      (bind _returnenemies (`self.RandomSpawnEnemies` SpawnLocation)))
    (:`then_3`
      (bind _returnvalue (`|SpawnActorFromClass` "/Game/InfiniteMatrix/Blueprints/BP_Tunnel.BP_Tunnel_C" (`KismetMathLibrary.MakeTransform` SpawnLocation) "Undefined" "MultiplyWithRoot" null null))
      (bind _output_get (set `self.NewestTunnel` _returnvalue))
      (set `/Game/InfiniteMatrix/Blueprints/BP_Tunnel.TunnelSpawner` self _output_get)
      (`/Game/InfiniteMatrix/Blueprints/BP_Tunnel.RandomizeWall` _output_get)
      (set `/Game/InfiniteMatrix/Blueprints/BP_Tunnel.HealthPack` _healthpack _returnvalue)
      (set `/Game/InfiniteMatrix/Blueprints/BP_Tunnel.SlowDown` _slowdown _returnvalue)
      (set `/Game/InfiniteMatrix/Blueprints/BP_Tunnel.Enemies` _returnenemies _returnvalue))))

(fn `SpawnTunnelAtSpawnPoint`
  (`self.SpawnTunnel` (`SceneComponent.K2_GetComponentLocation` (`/Game/InfiniteMatrix/Blueprints/BP_Tunnel.SpawnPoint` (`self.NewestTunnel`)))))

(fn `UserConstructionScript`)